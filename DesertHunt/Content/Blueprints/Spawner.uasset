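; Spawner actor that places a single Coin at a random point around itself when play begins.
; BeginPlay calls Spawn, which offsets X and Y by a random amount within the Range variable and picks Z from slightly below to well above the actor's location.
; Overlap and Tick events are unused, so it spawns only once.
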(event EventBeginPlay
  (CallFunction|Spawn))

(event Collision|EventActorBeginOverlap
  (params (OtherActor :type Actor%20Object%20Reference)))

(event EventTick
  (params (DeltaSeconds :type Float%20%28single-precision%29)))

(fn ConstructionScript)

(fn Spawn
  (bind _returnvalue (Transformation|GetActorLocation))
  (bind _returnvalue_2 (Transformation|GetActorLocation))
  (bind _returnvalue_3 (Transformation|GetActorLocation))
  (bind _range (Variables|Default|Getrange))
  (Game|SpawnActorfromClass "/Game/coin.coin_C" (Math|Transform|MakeTransform (Math|Vector|MakeVector (Math|Random|RandomFloatinRange (- (.x _returnvalue_2) _range) (+ (.x _returnvalue_2) _range)) (Math|Random|RandomFloatinRange (- (.y _returnvalue) _range) (+ (.y _returnvalue) _range)) (Math|Random|RandomFloatinRange (- (.z _returnvalue_3) 1e+02) (+ (.z _returnvalue_3) 2e+03))) "0, 0, 0" "1.000000,1.000000,1.000000") "Undefined" "MultiplyWithRoot" 0 0))