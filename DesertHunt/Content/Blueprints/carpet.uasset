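; Flying carpet actor that the player steers through Enhanced Input and that also checks the level's win and lose conditions.
; Inputs nudge it up below a height ceiling, down, or horizontally using the follow camera's forward vector as a local-space offset.
; Tick opens "Hell" if the character falls far below the carpet, otherwise "Won" once their Score reaches three.
; The ControlCarpet flag only triggers a debug print and does not gate movement.
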(event Input|EnhancedActionEvents|EnhancedInputActioncarpControl
  (params (ActionValue :type Boolean) (ElapsedSeconds :type Float%20%28double-precision%29) (TriggeredSeconds :type Float%20%28double-precision%29) (InputAction :type Input%20Action%20Object%20Reference :default "/Game/CarpControl/carpControl.carpControl"))
  (Variables|Default|SetcontrolCarpet true)
  (if (Variables|Default|GetcontrolCarpet)
    (Development|PrintString "carpet")))

(event Input|EnhancedActionEvents|EnhancedInputActionFly
  (params (ActionValue :type Boolean) (ElapsedSeconds :type Float%20%28double-precision%29) (TriggeredSeconds :type Float%20%28double-precision%29) (InputAction :type Input%20Action%20Object%20Reference :default "/Game/CarpControl/Fly.Fly"))
  (if (<= (.z (.location (Transformation|GetActorTransform self))) -8.09e+03)
    (Class|Actor|AddActorLocalTransform (Math|Conversions|ToTransform(Vector) "0.000000,0.000000,100.000000") false false)))

(event Input|EnhancedActionEvents|EnhancedInputActionflyforward
  (params (ActionValue :type Boolean) (ElapsedSeconds :type Float%20%28double-precision%29) (TriggeredSeconds :type Float%20%28double-precision%29) (InputAction :type Input%20Action%20Object%20Reference :default "/Game/CarpControl/flyforward.flyforward"))
  (bind _asbp_third_person_character (Utilities|Casting|CastToBP_ThirdPersonCharacter (Game|GetPlayerCharacter 0)))
  (Class|Actor|AddActorLocalTransform (Math|Conversions|ToTransform(Vector) (* (Math|Vector|GetForwardVector (Variables|/Game/ThirdPerson/Blueprints/BP_ThirdPersonCharacter.BP_ThirdPersonCharacter_C|GetFollowCamera _asbp_third_person_character)) "200.000000,200.000000,0.000000")) false false))

(event Input|EnhancedActionEvents|EnhancedInputActiondrop
  (params (ActionValue :type Boolean) (ElapsedSeconds :type Float%20%28double-precision%29) (TriggeredSeconds :type Float%20%28double-precision%29) (InputAction :type Input%20Action%20Object%20Reference :default "/Game/CarpControl/drop.drop"))
  (Class|Actor|AddActorLocalTransform (Math|Conversions|ToTransform(Vector) "0.000000,0.000000,-100.000000") false false))

(event EventBeginPlay
  (bind _returnvalue (Game|GetPlayerController 0))
  (Input|EnableInput _returnvalue)
  (bind _asplayer_controller (Utilities|Casting|CastToPlayerController _returnvalue))
  (Input|AddMappingContext (PlayerController|LocalPlayerSubsystems|GetEnhancedInputLocalPlayerSubsystem _asplayer_controller) "/Game/CarpControl/flymap.flymap" 0 "(bIgnoreAllPressedKeysUntilRelease=True,bForceImmediately=False,bNotifyUserSettings=False)")
  (Variables|Default|SetcontrolCarpet false))

(event EventTick
  (params (DeltaSeconds :type Float%20%28single-precision%29))
  (bind _returnvalue (Actor|GetActorOfClass "/Game/ThirdPerson/Blueprints/BP_ThirdPersonCharacter.BP_ThirdPersonCharacter_C"))
  (if (> (- (.z (Transformation|GetActorLocation)) (.z (Transformation|GetActorLocation _returnvalue))) 2e+03)
    (Game|OpenLevel(byName) "Hell")
    (Viewport|RemoveAllWidgets)
    (else
      (bind _returnvalue_2 (Actor|GetActorOfClass "/Game/ThirdPerson/Blueprints/BP_ThirdPersonCharacter.BP_ThirdPersonCharacter_C"))
      (if (>= (Variables|/Game/ThirdPerson/Blueprints/BP_ThirdPersonCharacter.BP_ThirdPersonCharacter_C|Getscore _returnvalue_2) 3)
        (Viewport|RemoveAllWidgets)
        (Game|OpenLevel(byName) "Won")))))

(event Collision|EventActorBeginOverlap
  (params (OtherActor :type Actor%20Object%20Reference)))

(fn ConstructionScript)